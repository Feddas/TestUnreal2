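; BP_PickUpSocket is a pickup actor whose static mesh can be attached to a socket on another component.
; Its PickUpSocket event takes a target component and socket name, then attaches the StaticMesh there with location, rotation and scale snapped to the target.
; When the attachment succeeds, the mesh's collision is disabled.
; Only the mesh component is reparented, and the actor has no other active logic.
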(event `/Game/dma226wk2/Blueprints/BPI_PickUpSocket.PickUpSocket`
  (params (ComponentRef :type "SceneComponent Object Reference") (Socket :type Name))
  (bind _returnvalue (`SceneComponent.K2_AttachToComponent` (`self.StaticMesh`) ComponentRef Socket "SnapToTarget" "SnapToTarget" "SnapToTarget" true))
  (if _returnvalue
    (`PrimitiveComponent.SetCollisionEnabled` (`self.StaticMesh`) "NoCollision")))

(fn `UserConstructionScript`
  (`parent.UserConstructionScript`))